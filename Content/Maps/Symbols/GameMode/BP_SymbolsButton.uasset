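; BP_SymbolsButton is an interactable button in the Symbols map that carries a numeric bomb symbol.
; The construction script writes the button's Symbol onto its text render component.
; On Interact, it reads the player's symbol from the character's Symbols component and prints it alongside the selected one.
; It only prints both values, with no comparison or game-state change.
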(event `/Game/FirstPerson/Blueprints/BPI_Interact.Interact`
  (params (FirstPersonCharacter :type "/Game/FirstPerson/Blueprints/BP_FirstPersonCharacter Object Reference"))
  (`KismetSystemLibrary.PrintString` (`KismetTextLibrary.Conv_TextToString` (`|FormatText` "The player has symbol {Symbol} and you selected {Bomb symbol}" (`/Game/Maps/Symbols/GameMode/Symbols.Symbol` (`self.GetComponentByClass` FirstPersonCharacter "/Game/Maps/Symbols/GameMode/Symbols.Symbols_C")) (`self.Symbol`)))))

(fn `UserConstructionScript`
  (`TextRenderComponent.K2_SetText` (`self.TextRender`) (`KismetTextLibrary.Conv_IntToText` (`self.Symbol`))))