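; GM_Symbols is the game mode for the Symbols map, which gives each first-person character a Symbols component, apparently a collar.
; BeginPlay and NewCollar share a five-second delay, then call ServerAddComponent on every BP_FirstPersonCharacter.
; Removed loops over those characters, only removing Symbols as a tick prerequisite rather than destroying it, and calls NewCollar inside the loop.
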(event `New Collar`
  (`KismetSystemLibrary.Delay` 5.0 :!label _label)
  (bind _outactors (`GameplayStatics.GetAllActorsOfClass` "/Game/FirstPerson/Blueprints/BP_FirstPersonCharacter.BP_FirstPersonCharacter_C"))
  (for _array_element _outactors
    (`/Game/FirstPerson/Blueprints/BP_FirstPersonCharacter.Server_AddComponent` _array_element "/Game/Maps/Symbols/GameMode/Symbols.Symbols_C")))

(event `self.ReceiveBeginPlay`
  (goto _label))

(event `Removed`
  (bind _outactors (`GameplayStatics.GetAllActorsOfClass` "/Game/FirstPerson/Blueprints/BP_FirstPersonCharacter.BP_FirstPersonCharacter_C"))
  (for _array_element _outactors
    (`self.RemoveTickPrerequisiteComponent` _array_element (`self.GetComponentByClass` _array_element "/Game/Maps/Symbols/GameMode/Symbols.Symbols_C"))
    (`self.New Collar`)))

(fn `UserConstructionScript`)